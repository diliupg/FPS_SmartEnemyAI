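; Melee enemy Blueprint that carries a sword and can attack, equip or sheathe it, and randomly block incoming blockable damage.
; Montage notifies move the spawned sword between sheath and hand sockets, and attacks are uninterruptable until the montage ends.
; Incoming blockable hits may start a timed block through the HealthComponent, with an impact montage on a successful block.
; Dispatchers report equip, unequip and block end, the latter used by the Behavior Tree.
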(event OnBlocked(HealthComponent)
  (params (CanBeParried :type Boolean))
  ;[0.1166 0.06746 0.1927] Blocking
  (Variables|Default|SetBlockingState "NewEnumerator2")
  (Utilities|Time|ClearandInvalidateTimerbyHandle (Variables|Default|GetHoldBlockTime))
  (Animation|Montage|PlayMontage (Variables|Character|GetMesh) "/Game/FPSGame/NPC/EnemyMeshes/EnemyBase/Animations/Montages/Montage_Great_Sword_Impact.Montage_Great_Sword_Impact"
    (:OnCompleted
      _)
    (:OnInterrupted
      _))
  (CallFunction|EndBlock))

(event Custom|StartBlock
  ;[0.1166 0.06746 0.1927] Blocking
  (Utilities|Time|ClearandInvalidateTimerbyHandle (Variables|Default|GetHoldBlockTime))
  (Components|Movement|StopMovementImmediately (Variables|Character|GetCharacterMovement))
  (Variables|/Game/FPSGame/DamageSystemDG/HealthComponent.HealthComponent_C|SetIsBlocking (Variables|Default|GetHealthComponent) true)
  (Variables|Default|SetBlockingState "NewEnumerator1")
  (bind _returnvalue (Utilities|Time|SetTimerbyEvent (EventDispatchers|CreateEvent :!event Custom|EndBlock) 2.0))
  (Variables|Default|SetHoldBlockTime _returnvalue))

(event Custom|EndBlock
  ;[0.1166 0.06746 0.1927] Blocking
  (Variables|/Game/FPSGame/DamageSystemDG/HealthComponent.HealthComponent_C|SetIsBlocking (Variables|Default|GetHealthComponent) false)
  (Variables|Default|SetBlockingState "NewEnumerator0")
  ;;[0.04504 0.1562 0.0405] event dispatch created and called from here which is accessed in the BT(Behaviour Tree)
  (Default|CallOnBlockEnded))

(event EventBeginPlay
  (|CallParentFunction)
  (bind _returnvalue (Game|SpawnActorfromClass "/Game/FPSGame/NPC/EnemyWeapons/BP_WeaponSword.BP_WeaponSword_C" (Transformation|GetActorTransform) "Undefined" 0 0))
  (bind _output_get (Variables|Default|SetWeaponActor _returnvalue))
  (Transformation|AttachComponentToComponent _output_get (Variables|Character|GetMesh) "SwordSheathSocket" "SnapToTarget" "SnapToTarget" "SnapToTarget" true))

(event EventUnEquipWeapon
  (bind _notifyname (Animation|Montage|PlayMontage (Variables|Character|GetMesh) "/Game/FPSGame/NPC/EnemyMeshes/EnemyBase/Animations/Montages/Sword_Sheath_Montage.Sword_Sheath_Montage")
    (:OnCompleted
      (Default|CallOnWeaponUnEquipped))
    (:OnNotifyBegin
      (switch name _notifyname
        (:SheathSword
          (Variables|Default|SetIsWeildingweapon false)
          (Transformation|AttachComponentToComponent (Variables|Default|GetWeaponActor) (Variables|Character|GetMesh) "SwordSheathSocket" "SnapToTarget" "SnapToTarget" "SnapToTarget" true))))))

(event EventEquipWeapon
  (bind _notifyname (Animation|Montage|PlayMontage (Variables|Character|GetMesh) "/Game/FPSGame/NPC/EnemyMeshes/EnemyBase/Animations/Montages/Sword_Weild_Montage.Sword_Weild_Montage")
    (:OnCompleted
      (Default|CallOnWeaponEquipped))
    (:OnNotifyBegin
      (switch name _notifyname
        (:WithdrawSword
          (Transformation|AttachComponentToComponent (Variables|Default|GetWeaponActor) (Variables|Character|GetMesh) "SwordSocket" "SnapToTarget" "SnapToTarget" "SnapToTarget" true)
          (Variables|Default|SetIsWeildingweapon true))))))

(event EventAttack
  (params (AttackTarget :type Actor%20Object%20Reference))
  (|CallParentFunction AttackTarget)
  (Animation|Montage|PlayMontage (Variables|Character|GetMesh) "/Game/FPSGame/NPC/EnemyMeshes/EnemyBase/Animations/Montages/Sword_Attack_Combo_CL_Heavy_Montage.Sword_Attack_Combo_CL_Heavy_Montage"
    (:then
      ;[0.1583 0.2917 0.04237] Can't be interrupted if atrtacking
      (Variables|/Game/FPSGame/DamageSystemDG/HealthComponent.HealthComponent_C|SetIsInterruptable (Variables|Default|GetHealthComponent) false))
    (:OnCompleted
      (CallFunction|AttackEnd AttackTarget :!label _label)
      (Variables|/Game/FPSGame/DamageSystemDG/HealthComponent.HealthComponent_C|SetIsInterruptable (Variables|Default|GetHealthComponent) true))
    (:OnInterrupted
      (goto _label))))

(fn ConstructionScript
  (|CallParentFunction))

(fn TakeDamageBPID
  (params (DamageInfo :type S%20Damage%20Info%20Structure) (DamageCauser :type Actor%20Object%20Reference))
  (if (Utilities|Struct|BreakS_DamageInfo DamageInfo)
    (CallFunction|TrytoBlock))
  (Default|TakeDamageHC (Variables|Default|GetHealthComponent) DamageInfo DamageCauser)
  (return false))

(fn TrytoBlock
  (if (<= (Math|Random|RandomFloat) (Variables|Default|GetBlockChance))
    (CallFunction|StartBlock)))