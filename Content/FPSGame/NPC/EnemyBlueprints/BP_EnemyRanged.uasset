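; Ranged enemy character that spawns a rifle on BeginPlay, attaches it to its mesh socket and fires at its AI target.
; Attack plays a hip-fire montage whose notify line-traces from the weapon to the AI controller's target.
; An unblocked trace applies fixed damage to a tagged player, and montage end or interruption signals attack end.
; It also supplies movement speeds per state and its ideal attack and defend range.
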(event EventBeginPlay
  (|CallParentFunction)
  (CallFunction|EquipWeapon)
  (Variables|/Game/FPSGame/DamageSystemDG/HealthComponent.HealthComponent_C|SetHealthReductionSpeed (Variables|Default|GetHealthComponent) (Variables|Default|GetNewHealthRedSpeed)) ; Set the health reduction speed individually
)

(event EventEquipWeapon
  (bind _returnvalue (Game|SpawnActorfromClass "/Game/FPSGame/NPC/EnemyWeapons/BP_WeaponRifle.BP_WeaponRifle_C" (Math|Transform|MakeTransform "0, 0, 0") "Undefined" 0 0))
  (bind _output_get (Variables|Default|SetWeaponActor _returnvalue))
  (Transformation|AttachComponentToComponent _output_get (Variables|Character|GetMesh) "RifleSocket" "SnapToTarget" "SnapToTarget" "SnapToTarget" true)
  (Variables|Default|SetIsWeildingweapon true)
  (Default|CallOnWeaponEquipped))

(event EventAttack
  (Variables|Default|SetAttacking true)
  (bind _notifyname (Animation|Montage|PlayMontage (Variables|Character|GetMesh) "/Game/FPSGame/NPC/EnemyMeshes/EnemyRanged/Animations/AM_Fire_Rifle_Hip.AM_Fire_Rifle_Hip")
    (:OnCompleted
      (Default|CallOnAttackEnd :!label _label)
      (Variables|Default|SetAttacking false))
    (:OnInterrupted
      (goto _label))
    (:OnNotifyBegin
      (switch name _notifyname
        (:Fire
          (bind _asaic_enemy_base (Utilities|Casting|CastToAIC_EnemyBase (AI|GetAIController self)))
          (bind _attack_target (Variables|/Game/FPSGame/NPC/AI/AIC/AIC_EnemyBase.AIC_EnemyBase_C|GetAttack%20Target _asaic_enemy_base) ; Validated get
            (:then
              (bind _returnvalue (Collision|LineTraceByChannel (Transformation|GetActorLocation (Variables|Default|GetWeaponActor)) (Transformation|GetActorLocation _attack_target) "TraceTypeQuery1" false 0 "None" true "(R=1.000000,G=0.000000,B=0.000000,A=1.000000)" "(R=0.000000,G=1.000000,B=0.000000,A=1.000000)" 15.0))
              (if (not _returnvalue)
                (bind _asbp_fp_player (Utilities|Casting|CastToBP_FP_Player _attack_target))
                (if (Actor|ActorHasTag _asbp_fp_player "player")
                  (Default|TakeDamageBPID _asbp_fp_player (Utilities|Struct|MakeS_DamageInfo 11.0 "NewEnumerator2" "NewEnumerator1") self))))
            (:else)))))))

(event EventTick
  (params (DeltaSeconds :type Float%20%28single-precision%29)))

(fn ConstructionScript
  (|CallParentFunction))

(fn SetMovementSpeed
  (params (Speed :type E_MovementSpeed%20Enum :default "NewEnumerator0"))
  (bind _output_get (Variables|/Script/Engine.CharacterMovementComponent|SetMaxWalkSpeed (Variables|Character|GetCharacterMovement) (Utilities|Select :Index Speed :NewEnumerator0 0.0 :NewEnumerator1 2.5e+02 :NewEnumerator2 4e+02 :NewEnumerator3 5e+02)))
  (return _output_get))

(fn GetIdealRange
  (return 6e+02 6e+02))